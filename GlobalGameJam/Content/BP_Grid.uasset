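; Clickable grid cell that lets the player trace a path cell by cell, by clicking or by hovering while NowClick is set on the player controller.
; It flags the move with StopMove when thin-wall maps or stone locations on the controller block it.
; A collapsed graph clears that flag or checks orthogonal adjacency on a five-wide numbered grid with row-edge handling, feeding the controller's LastHit and AnimGrid.
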(event OnClicked(Box)
  (params (TouchedComponent :type Primitive%20Component%20Object%20Reference) (ButtonPressed :type Key%20Structure :default "None"))
  (bind _returnvalue (Game|GetPlayerController 0))
  (bind _asmouse_playaer_controller (Utilities|Casting|CastToMouse_PlayaerController _returnvalue))
  (if (.ReturnValue (Utilities|Map|Find (Variables|/Game/Mouse_PlayaerController.Mouse_PlayaerController_C|GetThin%20Wall%20Location _asmouse_playaer_controller) (Variables|/Game/Mouse_PlayaerController.Mouse_PlayaerController_C|GetLastHit _asmouse_playaer_controller)))
    (if (== (.Value (Utilities|Map|Find (Variables|/Game/Mouse_PlayaerController.Mouse_PlayaerController_C|GetThin%20Wall%20Location _asmouse_playaer_controller) (Variables|/Game/Mouse_PlayaerController.Mouse_PlayaerController_C|GetLastHit _asmouse_playaer_controller))) (Variables|Default|GetGimickNomber))
      (Variables|Default|SetStop%20Move true)
      (else
        (if (.ReturnValue (Utilities|Map|Find (Variables|/Game/Mouse_PlayaerController.Mouse_PlayaerController_C|GetThin%20Wall%20Location%200 _asmouse_playaer_controller) (Variables|/Game/Mouse_PlayaerController.Mouse_PlayaerController_C|GetLastHit _asmouse_playaer_controller))) :!label _label
          (if (== (.Value (Utilities|Map|Find (Variables|/Game/Mouse_PlayaerController.Mouse_PlayaerController_C|GetThin%20Wall%20Location%200 _asmouse_playaer_controller) (Variables|/Game/Mouse_PlayaerController.Mouse_PlayaerController_C|GetLastHit _asmouse_playaer_controller))) (Variables|Default|GetGimickNomber))
            (Variables|Default|SetStop%20Move true)))))
    (else
      (goto _label)))
  (for _array_element (Variables|/Game/Mouse_PlayaerController.Mouse_PlayaerController_C|GetStone%20Location _asmouse_playaer_controller)
    (if (== _array_element (Variables|Default|GetGimickNomber))
      (Variables|Default|SetStop%20Move true)))
  (if (Variables|Default|GetStop%20Move)
    (bind _gimicknomber (|CollapseGraph_0 _asmouse_playaer_controller _asmouse_playaer_controller :!label _label_2))
    (Variables|/Game/Mouse_PlayaerController.Mouse_PlayaerController_C|SetAnimGrid _asmouse_playaer_controller (Variables|Default|GetGimickNomber))
    (Variables|/Game/Mouse_PlayaerController.Mouse_PlayaerController_C|SetLastHit _asmouse_playaer_controller _gimicknomber)
    (else
      (goto _label_2 execute2))))

(event OnBeginCursorOver(Box)
  (params (TouchedComponent :type Primitive%20Component%20Object%20Reference))
  (bind _returnvalue (Game|GetPlayerController 0))
  (bind _asmouse_playaer_controller (Utilities|Casting|CastToMouse_PlayaerController _returnvalue))
  (if (Variables|/Game/Mouse_PlayaerController.Mouse_PlayaerController_C|GetNowClick _asmouse_playaer_controller)
    (if (.ReturnValue (Utilities|Map|Find (Variables|/Game/Mouse_PlayaerController.Mouse_PlayaerController_C|GetThin%20Wall%20Location _asmouse_playaer_controller) (Variables|/Game/Mouse_PlayaerController.Mouse_PlayaerController_C|GetLastHit _asmouse_playaer_controller)))
      (if (== (.Value (Utilities|Map|Find (Variables|/Game/Mouse_PlayaerController.Mouse_PlayaerController_C|GetThin%20Wall%20Location _asmouse_playaer_controller) (Variables|/Game/Mouse_PlayaerController.Mouse_PlayaerController_C|GetLastHit _asmouse_playaer_controller))) (Variables|Default|GetGimickNomber))
        (Variables|Default|SetStop%20Move true)
        (else
          (if (.ReturnValue (Utilities|Map|Find (Variables|/Game/Mouse_PlayaerController.Mouse_PlayaerController_C|GetThin%20Wall%20Location%200 _asmouse_playaer_controller) (Variables|/Game/Mouse_PlayaerController.Mouse_PlayaerController_C|GetLastHit _asmouse_playaer_controller))) :!label _label
            (if (== (.Value (Utilities|Map|Find (Variables|/Game/Mouse_PlayaerController.Mouse_PlayaerController_C|GetThin%20Wall%20Location%200 _asmouse_playaer_controller) (Variables|/Game/Mouse_PlayaerController.Mouse_PlayaerController_C|GetLastHit _asmouse_playaer_controller))) (Variables|Default|GetGimickNomber))
              (Variables|Default|SetStop%20Move true)))))
      (else
        (goto _label)))
    (for _array_element (Variables|/Game/Mouse_PlayaerController.Mouse_PlayaerController_C|GetStone%20Location _asmouse_playaer_controller)
      (if (== _array_element (Variables|Default|GetGimickNomber))
        (Variables|Default|SetStop%20Move true)))
    (if (Variables|Default|GetStop%20Move)
      (bind _gimicknomber (|CollapseGraph_0 _asmouse_playaer_controller _asmouse_playaer_controller :!label _label_2))
      (Variables|/Game/Mouse_PlayaerController.Mouse_PlayaerController_C|SetAnimGrid _asmouse_playaer_controller (Variables|Default|GetGimickNomber))
      (Variables|/Game/Mouse_PlayaerController.Mouse_PlayaerController_C|SetLastHit _asmouse_playaer_controller _gimicknomber)
      (else
        (goto _label_2 execute2)))))

(event Collision|EventActorBeginOverlap
  (params (OtherActor :type Actor%20Object%20Reference)))

(event EventTick
  (params (DeltaSeconds :type Float%20%28single-precision%29)))

(fn ConstructionScript)