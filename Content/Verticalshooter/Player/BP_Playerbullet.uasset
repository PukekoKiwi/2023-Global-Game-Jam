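; Player bullet actor for the vertical shooter, shown as one of two word sprites.
; On BeginPlay it picks a sprite at random and plays the bullet firing sound.
; Hit-query functions, apparently from a shared interface, identify it to other actors: BulletHit returns 1, while the player, Hanetuki and special-hit queries return zero or false.
; The graphs contain no movement or collision logic.
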(event EventBeginPlay
  (Rendering|Components|Sprite|SetSprite (Variables|Default|GetPaperSprite) (select (Math|Random|RandomBool) "/Game/Illust/word2_Sprite.word2_Sprite" "/Game/Illust/word1_Sprite.word1_Sprite"))
  (Audio|PlaySound2D "/Game/Sound/bullet.bullet" 1.0 1.0 0.0 0 0))

(event Collision|EventActorBeginOverlap
  (params (OtherActor :type Actor%20Object%20Reference)))

(event EventTick
  (params (DeltaSeconds :type Float%20%28single-precision%29)))

(fn ConstructionScript)

(fn BulletHit
  (return 1))

(fn HanetukiHit
  (return false))

(fn PlayerDamage
  (return 0.0))

(fn PlayerHit
  (return 0 0 0 false))

(fn SpecialHit
  (return false))