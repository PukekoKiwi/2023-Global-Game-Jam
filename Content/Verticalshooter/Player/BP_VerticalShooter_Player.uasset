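; Player pawn for a vertical shooter, handling world-axis movement, normal fire and a limited special shot.
; Pressing Shot spawns a BP_Playerbullet at once and opens a Tick gate that repeats fire on a fixed timer until release resets it.
; Special shot spends RemainingAmmunition on the first BP_ItemMaster found in the world, prints the count and spawns BP_specialbullet while ammo remains.
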(event Custom|Open
  (Utilities|FlowControl|Gate true) ; enters at Open
)

(event Custom|Close
  (Utilities|FlowControl|Gate true) ; enters at Close
)

(event EventTick
  (params (DeltaSeconds :type Float%20%28single-precision%29))
  (Utilities|FlowControl|Gate true
    (:Exit
      (Variables|Default|SetShotTime (+ DeltaSeconds (Variables|Default|GetShotTime)))
      (if (>= (Variables|Default|GetShotTime) 0.8)
        (Game|SpawnActorfromClass "/Game/Verticalshooter/Player/BP_Playerbullet.BP_Playerbullet_C" (Transformation|GetActorTransform) "Undefined" 0 0)
        (Variables|Default|SetShotTime 0.0)))))

(event Input|ActionEvents|InputActionShot
  (params (Key :type Key%20Structure :default "None"))
  ;[1 1 1] 通常射撃　conventional shooting
  (:Pressed
    (Game|SpawnActorfromClass "/Game/Verticalshooter/Player/BP_Playerbullet.BP_Playerbullet_C" (Transformation|GetActorTransform) "Undefined" 0 0)
    (CallFunction|Open))
  (:Released
    (CallFunction|Close)
    (Variables|Default|SetShotTime 0.0)))

(event Input|ActionEvents|InputActionspecialshot
  (params (Key :type Key%20Structure :default "None"))
  (:Pressed
    (bind _returnvalue (Actor|GetActorOfClass "/Game/Verticalshooter/item/BP_ItemMaster.BP_ItemMaster_C"))
    (Utilities|IsValid _returnvalue
      (:Is%20Valid
        (Development|PrintString (Utilities|String|ToString(Integer) (Variables|/Game/Verticalshooter/item/BP_ItemMaster.BP_ItemMaster_C|GetRemaining%20Ammunition _returnvalue)))
        (if (not (<= (Variables|/Game/Verticalshooter/item/BP_ItemMaster.BP_ItemMaster_C|GetRemaining%20Ammunition _returnvalue) 0))
          (Variables|/Game/Verticalshooter/item/BP_ItemMaster.BP_ItemMaster_C|SetRemaining%20Ammunition _returnvalue (- (Variables|/Game/Verticalshooter/item/BP_ItemMaster.BP_ItemMaster_C|GetRemaining%20Ammunition _returnvalue) 1))
          (Game|SpawnActorfromClass "/Game/Verticalshooter/Player/BP_specialbullet.BP_specialbullet_C" (Transformation|GetActorTransform) "Undefined" 0 0))))))

(event Input|AxisEvents|InputAxisMoveForward
  (params (AxisValue :type Float%20%28single-precision%29))
  ;[1 1 1] 移動Move
  (Pawn|Input|AddMovementInput "0,1.000000, 0" AxisValue false))

(event Input|AxisEvents|InputAxisMoveRight
  (params (AxisValue :type Float%20%28single-precision%29))
  ;[1 1 1] 移動Move
  (Pawn|Input|AddMovementInput "1.000000, 0, 0" AxisValue false))

(fn ConstructionScript)