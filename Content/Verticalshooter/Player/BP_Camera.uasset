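; BP_Camera is the camera actor for the vertical shooter, making itself player 0's view target on BeginPlay.
; Its construction script stores the actor location as StartPos and that location plus the GoalEdit offset as GoalPos.
; A delayed timeline lerp between the two positions is present but unconnected to any event, so the camera does not scroll as written.
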(event EventBeginPlay
  (Game|Player|SetViewTargetwithBlend (Game|GetPlayerController 0) self 0.0 "VTBlend_Linear" 0.0 false))

(event Collision|EventActorBeginOverlap
  (params (OtherActor :type Actor%20Object%20Reference)))

(event EventTick
  (params (DeltaSeconds :type Float%20%28single-precision%29)))

(fn ConstructionScript
  (bind _returnvalue (Transformation|GetActorLocation))
  (Variables|Default|SetStart_Pos _returnvalue)
  (Variables|Default|SetGoal_Pos (+ _returnvalue (Variables|Default|GetGoal_Edit))))