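; BP_ItemBase is a base item Blueprint for the vertical shooter, defining hit responses and a score penalty.
; Its Hit event checks the other actor's name against the hard-coded BlockingVolume_7 and, on a match, subtracts the passed Score from BP_VerticalShooter_Player's score.
; BulletHit, HanetukiHit, PlayerDamage, PlayerHit and SpecialHit are stubs returning zero or false, with PlayerHit exposing Otoshidama, Happygauge, Score and SpecialHit outputs.
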(event Custom|Hit
  (params (OtherActor :type Actor%20Object%20Reference) (Score :type Integer))
  (if (Utilities|Name|Equal(Name) (Utilities|String|StringToName (Utilities|GetObjectName OtherActor)) "BlockingVolume_7")
    (bind _asbp_vertical_shooter_player (Utilities|Casting|CastToBP_VerticalShooter_Player (Game|Player|GetPlayerPawn 0)))
    (Variables|/Game/Verticalshooter/Player/BP_VerticalShooter_Player.BP_VerticalShooter_Player_C|SetScore _asbp_vertical_shooter_player (- (Variables|/Game/Verticalshooter/Player/BP_VerticalShooter_Player.BP_VerticalShooter_Player_C|GetScore _asbp_vertical_shooter_player) Score))))

(event EventBeginPlay)

(event Collision|EventActorBeginOverlap
  (params (OtherActor :type Actor%20Object%20Reference)))

(fn ConstructionScript)

(fn BulletHit
  (return 0))

(fn HanetukiHit
  (return false))

(fn PlayerDamage
  (return 0.0))

(fn PlayerHit
  (return 0 0 0 false))

(fn SpecialHit
  (return false))