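; Relative enemy for the vertical shooter that patrols sideways with flipping flipbooks and periodically breaks off into a "hug" lunge.
; Chained timelines lerp between start and right/left goals set in the Construction Script, with Move flags marking the active leg.
; A three-second timer stops that leg for the lunge, whose end restarts the patrol and timer.
; Bullet overlaps on Box destroy the bullet and spawn BP_GrandparentsOtoshidama at the enemy's transform.
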(event OnComponentBeginOverlap(Box)
  (params (OverlappedComponent :type Primitive%20Component%20Object%20Reference) (OtherActor :type Actor%20Object%20Reference) (OtherComp :type Primitive%20Component%20Object%20Reference) (OtherBodyIndex :type Integer) (bFromSweep :type Boolean) (SweepResult :type Hit%20Result%20Structure%20%28by%20ref%29))
  (bind _attack (Class|HitInterface|BulletHit(Message) OtherActor))
  (if (> _attack 0)
    (Actor|DestroyActor OtherActor)
    (Game|SpawnActorfromClass "/Game/Verticalshooter/item/BP_GrandparentsOtoshidama.BP_GrandparentsOtoshidama_C" (Transformation|GetActorTransform) "Undefined" 0 0)))

(event Custom|hug
  (bind _returnvalue (Transformation|GetActorLocation))
  (if (Variables|Default|GetMoveA)
    (Utilities|FlowControl|Sequence
      (:then_0
        (bind _新規track_0 (Timeline|タイムライン_0 Stop)
          (:Update
            (Transformation|SetActorLocation (Math|Vector|Lerp(Vector) (Variables|Default|GetStartLocation) (Variables|Default|GetRIghtGoal) _新規track_0) false false))
          (:Finished
            (Variables|Default|SetMoveB true :!label _label)
            (Variables|Default|SetMoveA false)
            (Sprite|SetFlipbook (Variables|Default|GetPaperFlipbook) "/Game/Illust/relative_left1.relative_left1")
            (bind _新規track_0_2 (Timeline|タイムライン_1 PlayFromStart)
              (:Update
                (Transformation|SetActorLocation (Math|Vector|Lerp(Vector) (Variables|Default|GetRIghtGoal) (Variables|Default|GetLeftGoal) _新規track_0_2) false false))
              (:Finished
                (Variables|Default|SetMoveC true)
                (Variables|Default|SetMoveB false)
                (Sprite|SetFlipbook (Variables|Default|GetPaperFlipbook) "/Game/Illust/relative_right1.relative_right1")
                (bind _新規track_0_3 (Timeline|タイムライン_2 PlayFromStart)
                  (:Update
                    (Transformation|SetActorLocation (Math|Vector|Lerp(Vector) (Variables|Default|GetLeftGoal) (Variables|Default|GetRIghtGoal) _新規track_0_3) false false))
                  (:Finished
                    (goto _label))))))))
      (:then_1
        (bind _新規track_0_4 (Timeline|タイムライン_3 PlayFromStart)
          (:Update
            (Transformation|SetActorLocation (Math|Vector|Lerp(Vector) (Transformation|GetActorLocation) (+ _returnvalue (+ _returnvalue "0,1570.000000, 0")) _新規track_0_4) false false))
          (:Finished
            (Utilities|FlowControl|Sequence
              (:then_0
                (Utilities|Time|SetTimerbyEvent (delegate Custom|hug) 3.0)
                (Sprite|SetFlipbook (Variables|Default|GetPaperFlipbook) "/Game/Illust/relative_right1.relative_right1")
                (Variables|Default|SetMoveA true)
                (Timeline|タイムライン_0 PlayFromStart))
              (:then_1
                (if (Variables|Default|GetMoveA)
                  (Timeline|タイムライン_0 Play)
                  (elif (Variables|Default|GetMoveB)
                    (Timeline|タイムライン_1 Play)
                    (else
                      (Timeline|タイムライン_2 Play))))))))))
    (elif (Variables|Default|GetMoveB)
      (Utilities|FlowControl|Sequence
        (:then_0
          (Timeline|タイムライン_1 Stop))
        (:then_1
          (Timeline|タイムライン_3 PlayFromStart)))
      (else
        (Utilities|FlowControl|Sequence
          (:then_0
            (Timeline|タイムライン_2 Stop))
          (:then_1
            (Timeline|タイムライン_3 PlayFromStart)))))))

(event EventBeginPlay
  (Utilities|Time|SetTimerbyEvent (delegate Custom|hug) 3.0)
  (Sprite|SetFlipbook (Variables|Default|GetPaperFlipbook) "/Game/Illust/relative_right1.relative_right1")
  (Variables|Default|SetMoveA true)
  (bind _新規track_0 (Timeline|タイムライン_0 PlayFromStart)
    (:Update
      (Transformation|SetActorLocation (Math|Vector|Lerp(Vector) (Variables|Default|GetStartLocation) (Variables|Default|GetRIghtGoal) _新規track_0) false false))
    (:Finished
      (Variables|Default|SetMoveB true :!label _label)
      (Variables|Default|SetMoveA false)
      (Sprite|SetFlipbook (Variables|Default|GetPaperFlipbook) "/Game/Illust/relative_left1.relative_left1")
      (bind _新規track_0_2 (Timeline|タイムライン_1 PlayFromStart)
        (:Update
          (Transformation|SetActorLocation (Math|Vector|Lerp(Vector) (Variables|Default|GetRIghtGoal) (Variables|Default|GetLeftGoal) _新規track_0_2) false false))
        (:Finished
          (Variables|Default|SetMoveC true)
          (Variables|Default|SetMoveB false)
          (Sprite|SetFlipbook (Variables|Default|GetPaperFlipbook) "/Game/Illust/relative_right1.relative_right1")
          (bind _新規track_0_3 (Timeline|タイムライン_2 PlayFromStart)
            (:Update
              (Transformation|SetActorLocation (Math|Vector|Lerp(Vector) (Variables|Default|GetLeftGoal) (Variables|Default|GetRIghtGoal) _新規track_0_3) false false))
            (:Finished
              (goto _label))))))))

(fn ConstructionScript
  (bind _returnvalue (Transformation|GetActorLocation))
  (Variables|Default|SetStartLocation _returnvalue)
  (Variables|Default|SetRIghtGoal (+ _returnvalue (Variables|デフォルト|GetRightEdit)))
  (Variables|Default|SetLeftGoal (+ _returnvalue (Variables|Default|GetLeftEdit))))