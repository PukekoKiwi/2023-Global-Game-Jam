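; Hagoita (battledore) enemy for the vertical shooter that rallies BP_Hanetuki projectiles with the player.
; It serves one from BulletPoint once the player pawn is near, rechecking by looping timer and delay until then.
; Box overlaps with returning projectiles destroy and re-serve them, counting hits until it replaces itself with BP_Hagoitaandfeathers.
; Hit-response functions return fixed values, with only player damage non-zero.
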(event OnComponentBeginOverlap(Box)
  (params (OverlappedComponent :type Primitive%20Component%20Object%20Reference) (OtherActor :type Actor%20Object%20Reference) (OtherComp :type Primitive%20Component%20Object%20Reference) (OtherBodyIndex :type Integer) (bFromSweep :type Boolean) (SweepResult :type Hit%20Result%20Structure%20%28by%20ref%29))
  (bind _hithagoita (Class|HitInterface|HanetukiHit(Message) OtherActor))
  (if _hithagoita
    (Actor|DestroyActor OtherActor)
    (if (== (Variables|Default|GetPlayHanetuki) 4)
      (Game|SpawnActorfromClass "/Game/Verticalshooter/item/BP_Hagoitaandfeathers.BP_Hagoitaandfeathers_C" (Transformation|GetActorTransform) "Undefined" 0 0)
      (Actor|DestroyActor)
      (else
        (Game|SpawnActorfromClass "/Game/Verticalshooter/Enemy/BP_Hanetuki.BP_Hanetuki_C" (Transformation|GetWorldTransform (Variables|Default|GetBulletPoint)) "Undefined" 0 0)
        (Variables|Default|SetPlayHanetuki (+ (Variables|Default|GetPlayHanetuki) 1))))))

(event Custom|re-injection
  (if (not (Variables|Default|GetHanetukiNow))
    (Utilities|FlowControl|Delay 1.0)
    (if (and (< (Transformation|GetDistanceTo (Game|Player|GetPlayerPawn 0)) 1.2e+03) (not (Variables|Default|GetHanetukiNow)))
      (Game|SpawnActorfromClass "/Game/Verticalshooter/Enemy/BP_Hanetuki.BP_Hanetuki_C" (Transformation|GetWorldTransform (Variables|Default|GetBulletPoint)) "Undefined" 0 0)
      (Variables|Default|SetHanetukiNow true)
      (else
        (bind _returnvalue (Utilities|Time|SetTimerbyEvent (delegate Custom|re-injection) 0.01 true))))))

(event EventBeginPlay
  (if (and (< (Transformation|GetDistanceTo (Game|Player|GetPlayerPawn 0)) 1.2e+03) (not (Variables|Default|GetHanetukiNow)))
    (Game|SpawnActorfromClass "/Game/Verticalshooter/Enemy/BP_Hanetuki.BP_Hanetuki_C" (Transformation|GetWorldTransform (Variables|Default|GetBulletPoint)) "Undefined" 0 0)
    (Variables|Default|SetHanetukiNow true)
    (else
      (bind _returnvalue (Utilities|Time|SetTimerbyEvent (delegate Custom|re-injection) 0.01 true)))))

(fn ConstructionScript)

(fn BulletHit
  (return 0))

(fn HanetukiHit
  (return false))

(fn PlayerDamage
  (return 5.0))

(fn PlayerHit
  (return 0 0 0 false))

(fn SpecialHit
  (return false))