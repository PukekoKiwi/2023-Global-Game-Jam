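; BP_relative is a vertical-shooter enemy that patrols sideways as an animated flipbook and drops a BP_Otoshidama pickup.
; The construction script derives both patrol goals from editable offsets.
; Three chained timelines lerp it right, then loop between goals, swapping left/right flipbooks and setting Move flags.
; Box overlaps query BulletHitMessage for damage; positive hits call DestroyActor before subtracting HP, spawning the drop only at zero or below.
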(event OnComponentBeginOverlap(Box)
  (params (OverlappedComponent :type Primitive%20Component%20Object%20Reference) (OtherActor :type Actor%20Object%20Reference) (OtherComp :type Primitive%20Component%20Object%20Reference) (OtherBodyIndex :type Integer) (bFromSweep :type Boolean) (SweepResult :type Hit%20Result%20Structure%20%28by%20ref%29))
  (bind _attack (Class|HitInterface|BulletHit(Message) OtherActor))
  (if (> _attack 0)
    (Actor|DestroyActor)
    (Variables|Default|SetHP (- (Variables|Default|GetHP) _attack))
    (if (<= (Variables|Default|GetHP) 0)
      (Game|SpawnActorfromClass "/Game/Verticalshooter/item/BP_Otoshidama.BP_Otoshidama_C" (Transformation|GetActorTransform) "Undefined" 0 0)
      (Actor|DestroyActor))))

(event EventBeginPlay
  (Sprite|SetFlipbook (Variables|Default|GetPaperFlipbook) "/Game/Illust/relative_right1.relative_right1")
  (Variables|Default|SetMoveA true)
  (bind _新規track_0 (Timeline|タイムライン_0 PlayFromStart)
    (:Update
      (Transformation|SetActorLocation (Math|Vector|Lerp(Vector) (Variables|Default|GetStartLocation) (Variables|Default|GetRIghtGoal) _新規track_0) false false))
    (:Finished
      (Variables|Default|SetMoveB true)
      (Variables|Default|SetMoveA false)
      (Sprite|SetFlipbook (Variables|Default|GetPaperFlipbook) "/Game/Illust/relative_left1.relative_left1" :!label _label)
      (bind _新規track_0_2 (Timeline|タイムライン_1 PlayFromStart)
        (:Update
          (Transformation|SetActorLocation (Math|Vector|Lerp(Vector) (Variables|Default|GetRIghtGoal) (Variables|Default|GetLeftGoal) _新規track_0_2) false false))
        (:Finished
          (Variables|Default|SetMoveC true)
          (Variables|Default|SetMoveB false)
          (Sprite|SetFlipbook (Variables|Default|GetPaperFlipbook) "/Game/Illust/relative_right1.relative_right1")
          (bind _新規track_0_3 (Timeline|タイムライン_2 PlayFromStart)
            (:Update
              (Transformation|SetActorLocation (Math|Vector|Lerp(Vector) (Variables|Default|GetLeftGoal) (Variables|Default|GetRIghtGoal) _新規track_0_3) false false))
            (:Finished
              (goto _label))))))))

(fn ConstructionScript
  (bind _returnvalue (Transformation|GetActorLocation))
  (Variables|Default|SetStartLocation _returnvalue)
  (Variables|Default|SetRIghtGoal (+ _returnvalue (Variables|デフォルト|GetRightEdit)))
  (Variables|Default|SetLeftGoal (+ _returnvalue (Variables|Default|GetLeftEdit))))