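; Parent enemy Blueprint for a vertical shooter that handles bullet damage and death.
; When its Box collision begins overlapping an actor, it calls BulletHitMessage on that actor and treats a positive return value as damage.
; A hit destroys the other actor and reduces HP; once HP runs out, the enemy spawns BP_Otoshidama at its own transform and destroys itself.
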(event OnComponentBeginOverlap(Box)
  (params (OverlappedComponent :type Primitive%20Component%20Object%20Reference) (OtherActor :type Actor%20Object%20Reference) (OtherComp :type Primitive%20Component%20Object%20Reference) (OtherBodyIndex :type Integer) (bFromSweep :type Boolean) (SweepResult :type Hit%20Result%20Structure%20%28by%20ref%29))
  (bind _attack (Class|HitInterface|BulletHit(Message) OtherActor))
  (if (> _attack 0)
    (Actor|DestroyActor OtherActor)
    (Variables|Default|SetHP (- (Variables|Default|GetHP) _attack))
    (if (<= (Variables|Default|GetHP) 0)
      (Game|SpawnActorfromClass "/Game/Verticalshooter/item/BP_Otoshidama.BP_Otoshidama_C" (Transformation|GetActorTransform) "Undefined" 0 0)
      (Actor|DestroyActor))))

(fn ConstructionScript)