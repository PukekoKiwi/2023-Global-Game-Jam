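; BP_piledupsnow is a destructible piled-up snow enemy or obstacle in the vertical shooter.
; On Box overlap, a positive bullet-hit value from the other actor destroys that actor and reduces HP, destroying the snow once HP runs out.
; Hit-response functions return constants: the snow damages the player, accepts Hanetuki hits, and gives no pickup, score or special-hit response.
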(event OnComponentBeginOverlap(Box)
  (params (OverlappedComponent :type Primitive%20Component%20Object%20Reference) (OtherActor :type Actor%20Object%20Reference) (OtherComp :type Primitive%20Component%20Object%20Reference) (OtherBodyIndex :type Integer) (bFromSweep :type Boolean) (SweepResult :type Hit%20Result%20Structure%20%28by%20ref%29))
  (bind _attack (Class|HitInterface|BulletHit(Message) OtherActor))
  (if (> _attack 0)
    (Actor|DestroyActor OtherActor)
    (Variables|Default|SetHP (- (Variables|Default|GetHP) _attack))
    (if (<= (Variables|Default|GetHP) 0)
      (Actor|DestroyActor))))

(fn ConstructionScript)

(fn BulletHit
  (return 0))

(fn HanetukiHit
  (return true))

(fn PlayerDamage
  (return 5.0))

(fn PlayerHit
  (return 0 0 0 false))

(fn SpecialHit
  (return false))