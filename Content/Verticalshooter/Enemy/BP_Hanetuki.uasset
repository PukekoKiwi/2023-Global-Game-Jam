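; BP_Hanetuki is a hanetsuki shuttlecock projectile in the vertical shooter's enemy set, linked to BP_Hagoita.
; A bullet overlap resets its velocity along negative Y.
; It ignores the first non-bullet overlap; a later one clears HanetukiNow on the found BP_Hagoita and destroys the shuttlecock, after a short delay if one exists.
; Hit-query functions identify it as a hanetsuki, report fixed player damage and grant no rewards.
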(event OnComponentBeginOverlap(Box)
  (params (OverlappedComponent :type Primitive%20Component%20Object%20Reference) (OtherActor :type Actor%20Object%20Reference) (OtherComp :type Primitive%20Component%20Object%20Reference) (OtherBodyIndex :type Integer) (bFromSweep :type Boolean) (SweepResult :type Hit%20Result%20Structure%20%28by%20ref%29))
  (bind _attack (Class|HitInterface|BulletHit(Message) OtherActor))
  (if (> _attack 0)
    (Variables|/Script/Engine.MovementComponent|SetVelocity (Variables|Default|GetProjectileMovement) "0,-200.000000, 0")
    (elif (Variables|Default|Getfirst%20hit)
      (bind _returnvalue (Actor|GetActorOfClass "/Game/Verticalshooter/Enemy/BP_Hagoita.BP_Hagoita_C"))
      (Utilities|IsValid _returnvalue
        (:Is%20Valid
          (Variables|/Game/Verticalshooter/Enemy/BP_Hagoita.BP_Hagoita_C|SetHanetukiNow _returnvalue false)
          (Utilities|FlowControl|Delay 0.2)
          (Actor|DestroyActor))
        (:Is%20Not%20Valid
          (Actor|DestroyActor)))
      (else
        (Variables|Default|Setfirst%20hit true)))))

(fn ConstructionScript)

(fn BulletHit
  (return 0))

(fn HanetukiHit
  (return true))

(fn PlayerDamage
  (return 5.0))

(fn PlayerHit
  (return 0 0 0 false))

(fn SpecialHit
  (return false))