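; BP_spinningatop is a shooter spinning-top enemy that player bullets spin up by hitting its Left or Right trigger.
; Same-side hits keep a timer raising RotationTime; an opposite hit, or the one-second Stop timer, resets it.
; Tick swaps flipbook and Pawn collision (overlap spinning, block idle), and at the spin threshold spawns BP_coma, destroys itself and plays an explosion.
; Hit and damage functions return fixed values.
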(event OnComponentBeginOverlap(Right)
  (params (OverlappedComponent :type Primitive%20Component%20Object%20Reference) (OtherActor :type Actor%20Object%20Reference) (OtherComp :type Primitive%20Component%20Object%20Reference) (OtherBodyIndex :type Integer) (bFromSweep :type Boolean) (SweepResult :type Hit%20Result%20Structure%20%28by%20ref%29))
  (bind _attack (Class|HitInterface|BulletHit(Message) OtherActor))
  (if (> _attack 0)
    (Actor|DestroyActor OtherActor)
    (if (Variables|Default|GetCiroclingLeft)
      (CallFunction|Stop)
      (Utilities|Time|ClearandInvalidateTimerbyHandle (stale _returnvalue))
      (Utilities|Time|ClearandInvalidateTimerbyHandle (stale _returnvalue_2))
      (else
        (if (Variables|Default|GetCircling%20right)
          _
          (else
            (Variables|Default|SetCircling%20right true)
            (bind _returnvalue (Utilities|Time|SetTimerbyEvent (delegate Custom|TurnTime) 0.1 true))))
        (bind _returnvalue_2 (Utilities|Time|SetTimerbyEvent (delegate Custom|Stop) 1.0))))))

(event OnComponentBeginOverlap(Left)
  (params (OverlappedComponent :type Primitive%20Component%20Object%20Reference) (OtherActor :type Actor%20Object%20Reference) (OtherComp :type Primitive%20Component%20Object%20Reference) (OtherBodyIndex :type Integer) (bFromSweep :type Boolean) (SweepResult :type Hit%20Result%20Structure%20%28by%20ref%29))
  (bind _attack (Class|HitInterface|BulletHit(Message) OtherActor))
  (if (> _attack 0)
    (Actor|DestroyActor OtherActor)
    (if (Variables|Default|GetCircling%20right)
      (CallFunction|Stop)
      (Utilities|Time|ClearandInvalidateTimerbyHandle (stale _returnvalue))
      (Utilities|Time|ClearandInvalidateTimerbyHandle (stale _returnvalue_2))
      (else
        (if (Variables|Default|GetCiroclingLeft)
          _
          (else
            (Variables|Default|SetCiroclingLeft true)
            (bind _returnvalue (Utilities|Time|SetTimerbyEvent (delegate Custom|TurnTime) 0.1 true))))
        (bind _returnvalue_2 (Utilities|Time|SetTimerbyEvent (delegate Custom|Stop) 1.0))))))

(event Custom|Stop
  (Variables|Default|SetRotation%20time 0.0)
  (Variables|Default|SetCircling%20right false)
  (Variables|Default|SetCiroclingLeft false)
  (Utilities|Time|ClearandInvalidateTimerbyHandle (stale OnComponentBeginOverlap(Right) _returnvalue))
  (Utilities|Time|ClearandInvalidateTimerbyHandle (stale OnComponentBeginOverlap(Left) _returnvalue)))

(event Custom|TurnTime
  (Variables|Default|SetRotation%20time (+ (Variables|Default|GetRotation%20time) 0.1)))

(event EventTick
  (params (DeltaSeconds :type Float%20%28single-precision%29))
  (Utilities|FlowControl|Sequence
    (:then_0
      (if (> (Variables|Default|GetRotation%20time) 0.0)
        (Sprite|SetFlipbook (Variables|Default|GetPaperFlipbook) "/Game/Illust/top1.top1")
        (else
          (Sprite|SetFlipbook (Variables|Default|GetPaperFlipbook) "/Game/Illust/top2.top2"))))
    (:then_1
      (if (>= (Variables|Default|GetRotation%20time) 5.0)
        (Game|SpawnActorfromClass "/Game/Verticalshooter/item/BP_coma.BP_coma_C" (Transformation|GetActorTransform) "Undefined" 0 0)
        (Actor|DestroyActor)
        (Audio|PlaySound2D "/Game/Sound/explosion.explosion" 1.0 1.0 0.0 0 0)
        (elif (> (Variables|Default|GetRotation%20time) 0.0)
          (Collision|SetCollisionResponsetoChannel (Variables|Default|GetBox) "ECC_Pawn" "ECR_Overlap")
          (else
            (Collision|SetCollisionResponsetoChannel (Variables|Default|GetBox) "ECC_Pawn" "ECR_Block")))))))

(fn ConstructionScript)

(fn BulletHit
  (return 0))

(fn HanetukiHit
  (return true))

(fn PlayerDamage
  (return 5.0))

(fn PlayerHit
  (return 0 0 0 false))

(fn SpecialHit
  (return false))