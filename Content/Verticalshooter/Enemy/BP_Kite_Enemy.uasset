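; Kite enemy for a vertical shooter that drifts along a line and turns into a BP_kite when shot enough.
; Once the player comes within range, a looping timer steadily lowers Alpha, which Tick uses to lerp between the start and a construction-time goal.
; Bullet hits raise Alpha and briefly pause that timer; reaching full Alpha spawns BP_kite and destroys the enemy.
; Overlapping a specific blocking volume, matched by name, also destroys it.
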(event OnComponentBeginOverlap(Box)
  (params (OverlappedComponent :type Primitive%20Component%20Object%20Reference) (OtherActor :type Actor%20Object%20Reference) (OtherComp :type Primitive%20Component%20Object%20Reference) (OtherBodyIndex :type Integer) (bFromSweep :type Boolean) (SweepResult :type Hit%20Result%20Structure%20%28by%20ref%29))
  (if (Utilities|Enum|Equal(Enum) (Utilities|GetObjectName OtherActor) "BlockingVolume_7")
    (Actor|DestroyActor)
    (else
      (bind _attack (Class|HitInterface|BulletHit(Message) OtherActor))
      (if (> _attack 0)
        (Actor|DestroyActor OtherActor)
        (Utilities|Time|PauseTimerbyHandle (stale Custom|FallStart _returnvalue))
        (bind _output_get (Variables|Default|SetAlpha (+ (Variables|Default|GetAlpha) 0.2)))
        (if (>= _output_get 1.0)
          (Game|SpawnActorfromClass "/Game/Verticalshooter/item/BP_kite.BP_kite_C" (Transformation|GetActorTransform) "Undefined" 0 0)
          (Actor|DestroyActor)
          (else
            (Utilities|FlowControl|Delay 1.0)
            (Utilities|Time|UnpauseTimerbyHandle (stale Custom|FallStart _returnvalue))))))))

(event Custom|fall
  (Variables|Default|SetAlpha (- (Variables|Default|GetAlpha) 0.01)))

(event Custom|FallStart
  (if (< (Transformation|GetDistanceTo (Game|Player|GetPlayerPawn 0)) 1.5e+03)
    (Utilities|Time|ClearandInvalidateTimerbyHandle (stale EventBeginPlay _returnvalue))
    (bind _returnvalue (Utilities|Time|SetTimerbyEvent (delegate Custom|fall) 0.1 true))))

(event EventBeginPlay
  (bind _returnvalue (Utilities|Time|SetTimerbyEvent (delegate Custom|FallStart) 0.01 true)))

(event Collision|EventActorBeginOverlap
  (params (OtherActor :type Actor%20Object%20Reference)))

(event EventTick
  (params (DeltaSeconds :type Float%20%28single-precision%29))
  (Transformation|SetActorLocation (Math|Vector|Lerp(Vector) (Variables|Default|GetStartLocation) (Variables|Default|GetGoal) (Variables|Default|GetAlpha)) false false))

(fn ConstructionScript
  (bind _returnvalue (Transformation|GetActorLocation))
  (Variables|Default|SetStartLocation _returnvalue)
  (Variables|Default|SetGoal (+ _returnvalue (+ _returnvalue "0,-300.000000, 0"))))